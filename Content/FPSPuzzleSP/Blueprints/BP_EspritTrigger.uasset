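; End-portal trigger that stays hidden and inert until a Turn On signal reveals its cylinder, enables its box and plays a portal sound.
; Overlapping the box enables a second, larger box, switches game mode, freezes the archaeologist character, shows the cursor and starts a dialogue.
; Each EventDialogue call advances through a text array in a reused WBP_PortalDialogue widget, then removes it, hides the cursor and opens the linked door.
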(event OnComponentBeginOverlap(Box)
  (params (OverlappedComponent :type Primitive%20Component%20Object%20Reference) (OtherActor :type Actor%20Object%20Reference) (OtherComp :type Primitive%20Component%20Object%20Reference) (OtherBodyIndex :type Integer) (bFromSweep :type Boolean) (SweepResult :type Hit%20Result%20Structure%20%28by%20ref%29))
  (Collision|SetCollisionEnabled (Variables|Default|GetBigBox) "QueryOnly")
  (CallFunction|EspritDialogueBox))

(event Custom|Esprit_Dialogue_Box
  (bind _asbp_third_person_game_mode (Utilities|Casting|CastToBP_ThirdPersonGameMode (Game|GetGameMode)))
  (Default|Switchmode _asbp_third_person_game_mode)
  (bind _asbp_third_person_character (Utilities|Casting|CastToBP_ThirdPersonCharacter (Variables|Default|GetArcheologue)))
  (Variables|/Game/ThirdPerson/Blueprints/BP_ThirdPersonCharacter.BP_ThirdPersonCharacter_C|SetisEndportal _asbp_third_person_character true)
  (Variables|/Script/Engine.PlayerController|SetbShowMouseCursor (Game|GetPlayerController 0) true)
  (Pawn|Components|CharacterMovement|DisableMovement (Variables|/Script/Engine.Character|GetCharacterMovement _asbp_third_person_character))
  (CallFunction|EventDialogue))

(event EventTurn
  (params (Signal :type Enum_Signal%20Enum :default "NewEnumerator0"))
  (switch Utilities|FlowControl|Switch|SwitchonEnum_Signal Signal
    (:NewEnumerator0
      (Development|SetHiddeninGame (Variables|Default|GetCylinder) false false)
      (Collision|SetCollisionEnabled (Variables|Default|GetBox) "QueryOnly")
      (Audio|PlaySound2D "/Game/Sounds/SC_EndPortal.SC_EndPortal" 1.0 1.0 0.0 0 0))))

(event EventBeginPlay
  (Development|SetHiddeninGame (Variables|Default|GetCylinder) true false)
  (Collision|SetCollisionEnabled (Variables|Default|GetBox) "NoCollision")
  (Collision|SetCollisionEnabled (Variables|Default|GetBigBox) "NoCollision"))

(event EventEventDialogue
  (Development|PrintString "Hello")
  (Math|Integer|IncrementInt (Variables|Default|GetTextIndex)
    (:%20%20
      (if (< (Variables|Default|GetTextIndex) (Utilities|Array|Length (Variables|Default|GetText)))
        (Variables|Default|GetUI
          (:then
            _)
          (:else
            (bind _returnvalue (UserInterface|CreateWidget "/Game/Widgets/WBP_PortalDialogue.WBP_PortalDialogue_C" (Game|GetPlayerController 0)))
            (bind _output_get (Variables|Default|SetUI _returnvalue))
            (UserInterface|Viewport|AddtoViewport _output_get 0)))
        (Rendering|Components|TextRender|SetText (Variables|/Game/Widgets/WBP_PortalDialogue.WBP_PortalDialogue_C|GetSpeech (Variables|Default|GetUI)) (Utilities|Text|ToText(String) (Utilities|Array|Get(acopy) (Variables|Default|GetText) (Variables|Default|GetTextIndex))))
        (else
          (Widget|RemovefromParent (Variables|Default|GetUI))
          (Class|BISignal|OpenDoor(Message) (Variables|Default|GetDoor) "NewEnumerator0")
          (Variables|/Script/Engine.PlayerController|SetbShowMouseCursor (Game|GetPlayerController 0) false))))))

(fn ConstructionScript
  (Components|Box|SetBoxExtent (Variables|Default|GetBox) (Variables|Settings|GetScale) true))