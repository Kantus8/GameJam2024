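; Trigger actor that plays a two-part dialogue when the third-person character enters its DialogueBox.
; Overlap shows the mouse cursor, disables character movement and fires EventDialogue, which advances one line per call.
; It steps through Text in a WBP_Dialogue widget, then TextSpirit in a WBP_DialogueSpirit widget, creating each on demand.
; After the last spirit line it removes the widget, hides the cursor and restores walking.
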(event OnComponentBeginOverlap(DialogueBox)
  (params (OverlappedComponent :type Primitive%20Component%20Object%20Reference) (OtherActor :type Actor%20Object%20Reference) (OtherComp :type Primitive%20Component%20Object%20Reference) (OtherBodyIndex :type Integer) (bFromSweep :type Boolean) (SweepResult :type Hit%20Result%20Structure%20%28by%20ref%29))
  (bind _asbp_third_person_character (Utilities|Casting|CastToBP_ThirdPersonCharacter OtherActor))
  (Variables|/Script/Engine.PlayerController|SetbShowMouseCursor (Game|GetPlayerController 0) true)
  (Pawn|Components|CharacterMovement|DisableMovement (Variables|/Script/Engine.Character|GetCharacterMovement _asbp_third_person_character))
  (CallFunction|EventDialogue))

(event OnComponentEndOverlap(DialogueBox)
  (params (OverlappedComponent :type Primitive%20Component%20Object%20Reference) (OtherActor :type Actor%20Object%20Reference) (OtherComp :type Primitive%20Component%20Object%20Reference) (OtherBodyIndex :type Integer)))

(event EventBeginPlay)

(event Collision|EventActorBeginOverlap
  (params (OtherActor :type Actor%20Object%20Reference)))

(event EventTick
  (params (DeltaSeconds :type Float%20%28single-precision%29)))

(event EventEventDialogue
  (Math|Integer|IncrementInt (Variables|Default|GetTextIndex)
    (:%20%20
      (if (< (Variables|Default|GetTextIndex) (Utilities|Array|Length (Variables|Default|GetText)))
        (Variables|Default|GetUI
          (:then
            _)
          (:else
            (bind _returnvalue (UserInterface|CreateWidget "/Game/Widgets/WBP_Dialogue.WBP_Dialogue_C" (Game|GetPlayerController 0)))
            (bind _output_get (Variables|Default|SetUI _returnvalue))
            (UserInterface|Viewport|AddtoViewport _output_get 0)))
        (Rendering|Components|TextRender|SetText (Variables|/Game/Widgets/WBP_Dialogue.WBP_Dialogue_C|GetSpeech (Variables|Default|GetUI)) (Utilities|Text|ToText(String) (Utilities|Array|Get(acopy) (Variables|Default|GetText) (Variables|Default|GetTextIndex))))
        (else
          (Widget|RemovefromParent (Variables|Default|GetUI))
          (Math|Integer|IncrementInt (Variables|Default|GetTextIndexSpirit)
            (:%20%20
              (if (< (Variables|Default|GetTextIndexSpirit) (Utilities|Array|Length (Variables|Default|GetTextSpirit)))
                (Variables|Default|GetUISpirit
                  (:then
                    _)
                  (:else
                    (bind _returnvalue_2 (UserInterface|CreateWidget "/Game/Widgets/WBP_DialogueSpirit.WBP_DialogueSpirit_C" (Game|GetPlayerController 0)))
                    (bind _output_get_2 (Variables|Default|SetUISpirit _returnvalue_2))
                    (UserInterface|Viewport|AddtoViewport _output_get_2 0)))
                (Rendering|Components|TextRender|SetText (Variables|/Game/Widgets/WBP_DialogueSpirit.WBP_DialogueSpirit_C|GetSpeechSpirit (Variables|Default|GetUISpirit)) (Utilities|Text|ToText(String) (Utilities|Array|Get(acopy) (Variables|Default|GetTextSpirit) (Variables|Default|GetTextIndexSpirit))))
                (else
                  (Widget|RemovefromParent (Variables|Default|GetUISpirit))
                  (Variables|/Script/Engine.PlayerController|SetbShowMouseCursor (Game|GetPlayerController 0) false)
                  (Pawn|Components|CharacterMovement|SetMovementMode (Variables|/Script/Engine.Character|GetCharacterMovement (Game|GetPlayerCharacter 0)) "MOVE_Walking" 0))))))))))

(fn ConstructionScript)